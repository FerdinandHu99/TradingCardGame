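; Elevator down button that simulates descent by pushing the physics-driven floors upward instead of moving the elevator.
; WhenClick, unless ElevatorFloor is 0, impulses every UpFloorClass actor and the separate-class ButtonFloorClass floor, then calls Acceleration on each.
; Tick zeroes the velocity of those floors at ElevatorFloor 0, except while UpButton.IsCanImpulse is set, so upward travel is not cancelled.
; Floor classes differ per shaft and are assigned in the level.
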(event EventBeginPlay)

(event Collision|EventActorBeginOverlap
  (params (OtherActor :type Actor%20Object%20Reference)))

(event EventTick
  (params (DeltaSeconds :type Float%20%28single-precision%29))
  ;[1 1 1] 楼层超过上限时(楼层往上移动(电梯下降时))速度为零
  ;;[1 1 1] 防止让楼层往下移动(电梯上升时)速度也被置为零
  (if (not (Variables|/Game/Up_Down/BP_Up.BP_Up_C|GetisCanImpulse (Variables|Default|GetUpButton)))
    (if (== (Variables|/Game/Elevator/ElevatorBase.ElevatorBase_C|GetElevatorFloor (Variables|Default|GetElevator)) 0.0)
      (for _array_element (Variables|Default|GetFloorArray)
        (Physics|SetPhysicsLinearVelocity (Variables|/Game/Floor/FloorBase.FloorBase_C|GetStaticMesh _array_element) "0, 0, 0" false "None"))
      (bind _returnvalue (Actor|GetActorOfClass (Variables|Default|GetButtonFloorClass)))
      (Physics|SetPhysicsLinearVelocity (Variables|/Game/Floor/FloorBase.FloorBase_C|GetStaticMesh _returnvalue) "0, 0, 0" false "None"))))

(event EventWhenClick
  (bind _forcescale (Variables|Default|GetForceScale))
  (bind _force (Variables|Default|GetForce))
  (bind _forcedirec (Variables|Default|GetForceDirec))
  (bind _returnvalue (* _force _forcescale))
  (bind _returnvalue_2 (* _returnvalue _forcedirec))
  ;[1 1 1] 为每个楼层添加冲量,下面额外还要get一次是由于第一层和其它层有区分,不是同一个类
  (if (not (== (Variables|/Game/Elevator/ElevatorBase.ElevatorBase_C|GetElevatorFloor (Variables|Default|GetElevator)) 0.0))
    (bind _outactors (Actor|GetAllActorsOfClass (Variables|Default|GetUpFloorClass)))
    (bind _output_get (Variables|Default|SetFloorArray _outactors))
    (for _array_element _output_get
      (Physics|AddImpulse (Variables|/Game/Floor/FloorBase.FloorBase_C|GetStaticMesh _array_element) _returnvalue_2 "None" false)
      (Default|Acceleration _array_element))
    (bind _returnvalue_3 (Actor|GetActorOfClass (Variables|Default|GetButtonFloorClass)))
    (Physics|AddImpulse (Variables|/Game/Floor/FloorBase.FloorBase_C|GetStaticMesh _returnvalue_3) _returnvalue_2 "None" false)
    (Default|Acceleration _returnvalue_3)))

(fn ConstructionScript
  (|CallParentFunction))